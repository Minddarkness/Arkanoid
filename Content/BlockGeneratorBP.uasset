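; BlockGeneratorBP is an actor that fills a flat grid with BlockBP actors when play begins.
; Nested loops over X and Y offset each block by BlockSize from the generator's location along world X and Y, keeping its Z.
; Every block spawns regardless of collisions.
; Tick, overlap and construction logic are empty.
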(event `self.ReceiveBeginPlay`
  (bind (_returnvalue_x _returnvalue_y _returnvalue_z) (`KismetMathLibrary.BreakVector` (`self.K2_GetActorLocation`)))
  (for _index (range (+ (`self.X`) 1))
    (for _index_2 (range (+ (`self.Y`) 1))
      (`|SpawnActorFromClass` "/Game/BlockBP.BlockBP_C" (`KismetMathLibrary.MakeTransform` (`KismetMathLibrary.MakeVector` (+ _returnvalue_x (* _index (`self.Block Size`))) (+ _returnvalue_y (* _index_2 (`self.Block Size`))) _returnvalue_z)) "AlwaysSpawn" "OverrideRootScale" null null))))

(fn `UserConstructionScript`)